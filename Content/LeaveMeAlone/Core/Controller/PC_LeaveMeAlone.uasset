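; Player controller for LeaveMeAlone that handles the pause menu and the game-over screen.
; The Pause input pauses the game once, shows the pause widget and switches to UI-only input with a visible cursor.
; On possess it binds to the pawn's destroyed event, which shows the game-over widget and pauses the game.
; Unpausing is not handled in this controller.
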(event Custom|ShowGameOverScreen
  (bind _returnvalue (UserInterface|CreateWidget "/Game/LeaveMeAlone/Widgets/UI/WBP_GameOver.WBP_GameOver_C"))
  (UserInterface|Viewport|AddtoViewport _returnvalue 0)
  (Input|SetInputModeUIOnly self 0 "DoNotLock" false)
  (Variables|Default|SetbShowMouseCursor true))

(event Custom|OnPawnDeath
  (params (DestroyedActor :type Actor%20Object%20Reference))
  (CallFunction|ShowGameOverScreen)
  (Game|SetGamePaused true))

(event EventBeginPlay)

(event EventTick
  (params (DeltaSeconds :type Float%20%28single-precision%29)))

(event EventPossess
  (params (PossessedPawn :type Pawn%20Object%20Reference))
  (Game|BindEventtoOnDestroyed PossessedPawn (delegate Custom|OnPawnDeath)))

(event Input|ActionEvents|InputActionPause
  (params (Key :type Key%20Structure :default "None"))
  (:Pressed
    (if (not (Variables|Default|GetOnPause))
      (bind _output_get (Variables|Default|SetOnPause true))
      (Game|SetGamePaused _output_get)
      (bind _returnvalue (UserInterface|CreateWidget "/Game/LeaveMeAlone/Widgets/UI/WBP_Pause.WBP_Pause_C"))
      (bind _output_get_2 (Variables|Default|SetPauseWidget _returnvalue))
      (UserInterface|Viewport|AddtoViewport _output_get_2 0)
      (Input|SetInputModeUIOnly self _output_get_2 "DoNotLock" false)
      (Variables|Default|SetbShowMouseCursor true))))

(fn ConstructionScript)